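; NPC that speaks random dialogue lines and takes a dish delivery to end its turn.
; Talk shows a random Dialogue entry in a WB_Dialogue widget with a click sound, doing nothing when the roll equals the array length.
; Trigger_Zone treats an overlapping "Pollo"-tagged actor as the dish, clearing IsMyTurn and signalling turn finish; any end overlap hides the widget.
; AI movement between two destinations is present but never runs.
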(event `self.ReceiveBeginPlay`
  (bind _returnvalue (`|CreateWidget` "/Game/L_PruebasPlush/Dialogue/WB_Dialogue.WB_Dialogue_C"))
  (bind _output_get (set `self.UI` _returnvalue))
  (`UserWidget.AddToViewport` _output_get 0)
  (`Widget.SetVisibility` _output_get "Collapsed"))

(event `/Game/L_PruebasPlush/Dialogue/BPI_Dialogue.Talk`
  (bind _returnvalue (`KismetArrayLibrary.Array_Length` (`self.Dialogue`)))
  (set `self.Takl_Index` (`KismetMathLibrary.RandomIntegerInRange` 0 _returnvalue))
  (if (< (`self.Takl_Index`) _returnvalue)
    (bind _ui (`self.UI`)
      (:`then`
        (`Widget.SetVisibility` _ui "Visible"))
      (:`else`
        (bind _returnvalue_2 (`|CreateWidget` "/Game/L_PruebasPlush/Dialogue/WB_Dialogue.WB_Dialogue_C" (`GameplayStatics.GetPlayerController` 0)))
        (bind _output_get (set `self.UI` _returnvalue_2))
        (`UserWidget.AddToViewport` _output_get 0)))
    (`TextBlock.SetText` (`/Game/L_PruebasPlush/Dialogue/WB_Dialogue.Talk_Text` (`self.UI`)) (`KismetTextLibrary.Conv_StringToText` (`|GetArrayItem` (`self.Dialogue`) (`self.Takl_Index`))))
    (`GameplayStatics.PlaySound2D` "/Engine/VREditor/Sounds/UI/Click_on_Button.Click_on_Button" 1.0 1.0 0.0 null null)))

(event `self.Trigger_Zone.OnComponentEndOverlap`
  (params (OverlappedComponent :type "PrimitiveComponent Object Reference") (OtherActor :type "Actor Object Reference") (OtherComp :type "PrimitiveComponent Object Reference") (OtherBodyIndex :type Integer))
  (`Widget.SetVisibility` (`self.UI`) "Collapsed"))

(event `self.Trigger_Zone.OnComponentBeginOverlap`
  (params (OverlappedComponent :type "PrimitiveComponent Object Reference") (OtherActor :type "Actor Object Reference") (OtherComp :type "PrimitiveComponent Object Reference") (OtherBodyIndex :type Integer) (bFromSweep :type Boolean) (SweepResult :type "HitResult Structure (by ref)"))
  (if (`self.ActorHasTag` OtherActor "Pollo")
    (`self.ReceiveDish`)))

(fn `ReceiveDish`
  (set `self.IsMyTurn` false)
  (`self.TurnFinish`))

(fn `UserConstructionScript`)