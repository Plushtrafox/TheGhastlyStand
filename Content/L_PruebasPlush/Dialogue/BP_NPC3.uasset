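; BP_NPC3 is a talking NPC that also accepts a delivered dish when it is its turn.
; Talk picks a random index into its dialogue array and, when in range, shows that line in a WB_Dialogue widget with a click sound.
; Its trigger zone hides the widget on overlap end, and on a "Pollo"-tagged overlap during its turn calls ReceiveDish and destroys that actor.
; A two-stop AI movement sequence is present but disconnected.
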(event `self.ReceiveBeginPlay`
  (bind _returnvalue (`|CreateWidget` "/Game/L_PruebasPlush/Dialogue/WB_Dialogue.WB_Dialogue_C"))
  (bind _output_get (set `self.UI_0` _returnvalue))
  (`UserWidget.AddToViewport` _output_get 0)
  (`Widget.SetVisibility` _output_get "Collapsed"))

(event `self.Talk`
  (bind _returnvalue (`KismetArrayLibrary.Array_Length` (`self.Dialogue_0`)))
  (set `self.Takl_Index_0` (`KismetMathLibrary.RandomIntegerInRange` 0 _returnvalue))
  (if (< (`self.Takl_Index_0`) _returnvalue)
    (bind _ui_0 (`self.UI_0`)
      (:`then`
        (`Widget.SetVisibility` _ui_0 "Visible"))
      (:`else`
        (bind _returnvalue_2 (`|CreateWidget` "/Game/L_PruebasPlush/Dialogue/WB_Dialogue.WB_Dialogue_C" (`GameplayStatics.GetPlayerController` 0)))
        (bind _output_get (set `self.UI_0` _returnvalue_2))
        (`UserWidget.AddToViewport` _output_get 0)))
    (`TextBlock.SetText` (`/Game/L_PruebasPlush/Dialogue/WB_Dialogue.Talk_Text` (`self.UI_0`)) (`KismetTextLibrary.Conv_StringToText` (`|GetArrayItem` (`self.Dialogue_0`) (`self.Takl_Index_0`))))
    (`GameplayStatics.PlaySound2D` "/Engine/VREditor/Sounds/UI/Click_on_Button.Click_on_Button" 1.0 1.0 0.0 null null)))

(event `self.Trigger_Zone_0.OnComponentEndOverlap`
  (params (OverlappedComponent :type "PrimitiveComponent Object Reference") (OtherActor :type "Actor Object Reference") (OtherComp :type "PrimitiveComponent Object Reference") (OtherBodyIndex :type Integer))
  (`Widget.SetVisibility` (`self.UI_0`) "Collapsed"))

(event `self.Trigger_Zone_0.OnComponentBeginOverlap`
  (params (OverlappedComponent :type "PrimitiveComponent Object Reference") (OtherActor :type "Actor Object Reference") (OtherComp :type "PrimitiveComponent Object Reference") (OtherBodyIndex :type Integer) (bFromSweep :type Boolean) (SweepResult :type "HitResult Structure (by ref)"))
  (if (`self.ActorHasTag` OtherActor "Pollo")
    (if (`self.IsMyTurn`)
      (`self.ReceiveDish`)
      (`self.K2_DestroyActor` OtherActor))))

(fn `UserConstructionScript`)