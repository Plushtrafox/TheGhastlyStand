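; BP_Character is a character Blueprint with an unfinished click-to-grab prototype for physics objects.
; Left mouse press traces under the cursor and checks whether the hit component simulates physics, but neither branch does anything.
; The GrabComponentAtLocation node is unconnected, while mouse release calls ReleaseComponent on PhysicsHandle.
; Tick clears the PhysicsHandle reference, then sets its target to the origin, so dragging is non-functional.
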(event `Key|LeftMouseButton`
  (params (Key :type "Key Structure"))
  (bind (_hitresult _returnvalue) (`PlayerController.GetHitResultUnderCursorByChannel` (`GameplayStatics.GetPlayerController` 0) "TraceTypeQuery1" true))
  (:`Pressed`
    (if _returnvalue
      (if (`SceneComponent.IsSimulatingPhysics` (`.HitComponent` (`GameplayStatics.BreakHitResult` _hitresult)) "None")
        _)))
  (:`Released`
    (`PhysicsHandleComponent.ReleaseComponent` (`self.PhysicsHandle`))))

(event `self.ReceiveTick`
  (params (DeltaSeconds :type "Float (single-precision)"))
  (bind _output_get (set `self.PhysicsHandle` null))
  (`PhysicsHandleComponent.SetTargetLocation` _output_get (0.0 0.0 0.0)))

(fn `UserConstructionScript`)