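; Test player character with Enhanced Input movement and look, a physics-simulated mesh, player HUD, pause menu and countdown timer.
; E sends a dialogue message to overlapping NPCs, and a debug key grabs traced components.
; Drag traces from the camera to spend Cash on money-interface actors or grab physics bodies, holding them camera-relative via PhysicsHandle and a self-recalling delay loop.
; The game-over widget logic is unconnected.
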(event Custom|PickedUp
  (bind _camera (Variables|Default|GetCamera))
  ;[0.15 0.15 0.15 0.5] Updating Picked Up Object's Location
  (Utilities|Time|SetTimerbyEvent (delegate Custom|PickedUp) 0.02 true true)
  (Physics|Components|PhysicsHandle|SetTargetLocation (Variables|Default|GetPhysicsHandle) (+ (Transformation|GetWorldLocation _camera) (* (Math|Vector|GetForwardVector (Transformation|GetWorldRotation _camera)) 1e+02))))

(event Input|EnhancedActionEvents|EnhancedInputActionIA_MouselookPrueba
  (params (ActionValue :type Vector%202D%20Structure) (ElapsedSeconds :type Float%20%28double-precision%29) (TriggeredSeconds :type Float%20%28double-precision%29) (InputAction :type Input%20Action%20Object%20Reference :default "/Game/L_PruebasPlush/Inputs/Input/IA_MouselookPrueba.IA_MouselookPrueba"))
  (Pawn|Input|AddControllerYawInput (.x ActionValue))
  (Pawn|Input|AddControllerPitchInput (.y ActionValue)))

(event Input|EnhancedActionEvents|EnhancedInputActionIA_MovePrueba
  (params (ActionValue :type Vector%202D%20Structure) (ElapsedSeconds :type Float%20%28double-precision%29) (TriggeredSeconds :type Float%20%28double-precision%29) (InputAction :type Input%20Action%20Object%20Reference :default "/Game/L_PruebasPlush/Inputs/Input/IA_MovePrueba.IA_MovePrueba"))
  (|MoveSystem (.x ActionValue) (.y ActionValue)))

(event Input|EnhancedActionEvents|EnhancedInputActionIA_DragPrueba
  (params (ActionValue :type Boolean) (ElapsedSeconds :type Float%20%28double-precision%29) (TriggeredSeconds :type Float%20%28double-precision%29) (InputAction :type Input%20Action%20Object%20Reference :default "/Game/L_PruebasPlush/Inputs/Input/IA_DragPrueba.IA_DragPrueba"))
  (:Started
    (|Drag :!label _label))
  (:Completed
    (goto _label execute2)))

(event EventTick
  (params (DeltaSeconds :type Float%20%28single-precision%29))
  (Utilities|FlowControl|Delay 1.0)
  (if (== (Variables|Default|GetSeconds) 0)
    (if (not (== (Variables|Default|GetMinutes) 0))
      (Variables|Default|SetSeconds 0)
      (Variables|Default|SetMinutes (- (Variables|Default|GetMinutes) 1)))
    (else
      (Variables|Default|SetSeconds (- (Variables|Default|GetSeconds) 1)))))

(event EventBeginPlay
  (Physics|SetSimulatePhysics (Variables|Character|GetMesh) true)
  (bind _returnvalue (UserInterface|CreateWidget "/Game/L_PruebasPlush/UI/UI_Player.UI_Player_C"))
  (UserInterface|Viewport|AddtoPlayerScreen _returnvalue)
  (Variables|Default|SetPlayerUI _returnvalue))

(event Input|KeyboardEvents|DebugKeyE
  (params (Key :type Key%20Structure) (ActionValue :type Input%20Action%20Value%20Structure))
  (bind _camera (Variables|Default|GetCamera))
  (bind _returnvalue (Transformation|GetWorldLocation _camera))
  ;[0.15 0.15 0.15 0.5] Grabbing Function
  (:Pressed
    (bind (_outhit _returnvalue_2) (Collision|LineTraceByChannel _returnvalue (+ (* (Math|Vector|GetForwardVector (Transformation|GetWorldRotation _camera)) 5e+02) _returnvalue) "TraceTypeQuery1" false 0 "None"))
    (if _returnvalue_2
      (Physics|Components|PhysicsHandle|GrabComponentatLocationwithRotation (Variables|Default|GetPhysicsHandle) (.HitComponent (Collision|BreakHitResult _outhit)) "None" (Transformation|GetWorldLocation (.HitComponent (Collision|BreakHitResult _outhit))) "0, 0, 0")
      (Variables|Default|SetbIsGrabbing true)
      (CallFunction|PickedUp)))
  (:Released
    (if (Variables|Default|GetbIsGrabbing)
      (Physics|Components|PhysicsHandle|ReleaseComponent (Variables|Default|GetPhysicsHandle))
      (Variables|Default|SetbIsGrabbing true))))

(event Input|KeyboardEvents|E
  (params (Key :type Key%20Structure))
  (:Pressed
    (for _array_element (Collision|GetOverlappingActors "/Game/L_PruebasPlush/Dialogue/BP_NPC.BP_NPC_C" :!class /Script/Engine.Actor)
      (if (Utilities|DoesObjectImplementInterface _array_element "/Game/L_PruebasPlush/Dialogue/BPI_Dialogue.BPI_Dialogue_C")
        (Class|BPIDialogue|Talk(Message) _array_element)))))

(event Input|MouseEvents|RightMouseButton
  (params (Key :type Key%20Structure)))

(fn ConstructionScript)

(fn NewFunction0)

(event Custom|UpdateTargetRagdollLocation
  (Utilities|IsValid (Variables|Default|GetRagdollTarget)
    (:Is%20Valid
      (Physics|Components|PhysicsHandle|SetTargetLocation (Variables|Default|GetPhysicsHandle) (Math|Transform|TransformLocation (Transformation|GetWorldTransform (Variables|Default|GetCamera)) (Variables|Default|GetTargetLocation)))
      (Utilities|FlowControl|Delay 0.01)
      (CallFunction|UpdateTargetRagdollLocation))))

(event Input|EnhancedActionEvents|EnhancedInputActionIA_PauseGame
  (params (ActionValue :type Boolean) (ElapsedSeconds :type Float%20%28double-precision%29) (TriggeredSeconds :type Float%20%28double-precision%29) (InputAction :type Input%20Action%20Object%20Reference :default "/Game/L_PruebasPlush/Inputs/Input/IA_PauseGame.IA_PauseGame"))
  (bind _returnvalue (Game|GetPlayerController 0))
  (:Started
    (if (not (Variables|Default|Getis%20Paused%20Menu%20Opened?))
      (Variables|Default|Setis%20Paused%20Menu%20Opened? true)
      (bind _returnvalue_2 (UserInterface|CreateWidget "/Game/L_PruebasPlush/UI/UI_PauseMenu.UI_PauseMenu_C" _returnvalue))
      (bind _output_get (Variables|Default|SetPause%20Menu%20UI _returnvalue_2))
      (UserInterface|Viewport|AddtoViewport _output_get 0)
      (Input|SetInputModeGameandUI _returnvalue (Variables|Default|GetPause%20Menu%20UI) "DoNotLock" true false)
      (Variables|/Script/Engine.PlayerController|SetbShowMouseCursor (Game|GetPlayerController 0) true)
      (Game|SetGamePaused true)
      (else
        (Variables|Default|Setis%20Paused%20Menu%20Opened? false)
        (Widget|RemovefromParent (Variables|Default|GetPause%20Menu%20UI))
        (Game|SetGamePaused false)
        (Input|SetInputModeGameOnly _returnvalue false)
        (Variables|/Script/Engine.PlayerController|SetbShowMouseCursor (Game|GetPlayerController 0) false)))))