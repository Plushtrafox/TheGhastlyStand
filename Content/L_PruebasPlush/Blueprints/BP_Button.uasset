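; BP_Button is a pressable button actor that dispenses a test food actor when its SpendMoney event fires.
; SpendMoney plays a timeline that slides the Cube along its local Y axis as press feedback.
; When the timeline finishes, the Cube's Y resets to zero and BP_FoodPrueba spawns at SpawnLocation.
; Despite the event name, no money is checked or deducted here.
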(event `/Game/L_PruebasPlush/Blueprints/BPI_MoneySystem.SpendMoney`
  (bind _cube (`self.Cube`))
  (bind _cube_2 (`self.Cube`))
  (bind (_relativelocation_x _relativelocation_y _relativelocation_z) (`KismetMathLibrary.BreakVector` (`SceneComponent.RelativeLocation` _cube)))
  (bind (_relativelocation_x_2 _relativelocation_y_2 _relativelocation_z_2) (`KismetMathLibrary.BreakVector` (`SceneComponent.RelativeLocation` _cube_2)))
  (bind (_direction _floattrack) (`Timeline|TL_ButtonPressed` :!via `PlayFromStart`)
    (:`Update`
      (`SceneComponent.K2_SetRelativeLocation` _cube_2 (`KismetMathLibrary.MakeVector` _relativelocation_x_2 (* _floattrack 2.0) _relativelocation_z_2) false false))
    (:`Finished`
      (`SceneComponent.K2_SetRelativeLocation` _cube (`KismetMathLibrary.MakeVector` _relativelocation_x (* _floattrack 0.0) _relativelocation_z) false false)
      (`|SpawnActorFromClass` "/Game/L_PruebasPlush/Blueprints/BP_FoodPrueba.BP_FoodPrueba_C" (`self.SpawnLocation`) "AlwaysSpawn" "MultiplyWithRoot" null null))))

(fn `UserConstructionScript`)