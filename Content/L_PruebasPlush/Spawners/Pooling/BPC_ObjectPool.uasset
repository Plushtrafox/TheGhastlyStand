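; Actor component that serves as an object pool, pre-spawning actors for reuse.
; On BeginPlay, InizializePool spawns PoolSize instances of the PooledActor class and stores them in ActorsInPool.
; FindPooledActor is unfinished: it loops over the pool, but its branch is empty, the IsBeingUsed check is unconnected, and it returns no actor.
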(event `self.ReceiveBeginPlay`
  (`self.InizializePool`))

(fn `FindPooledActor`
  (for _array_element (`self.ActorsInPool`)
    (if true
      _)))

(fn `InizializePool`
  (for _ (range 1 (+ (`self.PoolSize`) 1))
    (bind _returnvalue (`|SpawnActorFromClass` (`self.PooledActor`) (`KismetMathLibrary.MakeTransform` (0.0 0.0 0.0)) "Undefined" "MultiplyWithRoot" null null))
    (`KismetArrayLibrary.Array_AddUnique` (`self.ActorsInPool`) _returnvalue)))